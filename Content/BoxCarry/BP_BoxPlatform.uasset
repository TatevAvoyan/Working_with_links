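; BP_BoxPlatform is a drop-off platform that takes the box a character is carrying.
; When a ThirdPersonCharacter overlaps its Box component, it stores that character's CurrentBoxCarrying as BoxOnPlatform and clears the character's reference.
; It then detaches the box and teleport-free moves it to the platform actor's location without sweeping.
; Debug strings report placement, empty-handed characters and non-character overlaps.
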(event OnComponentBeginOverlap(Box)
  (params (OverlappedComponent :type Primitive%20Component%20Object%20Reference) (OtherActor :type Actor%20Object%20Reference) (OtherComp :type Primitive%20Component%20Object%20Reference) (OtherBodyIndex :type Integer) (bFromSweep :type Boolean) (SweepResult :type Hit%20Result%20Structure%20%28by%20ref%29))
  (bind _asthird_person_character (Utilities|Casting|CastToThirdPersonCharacter OtherActor)
    (:then
      (Utilities|IsValid (Variables|/Game/ThirdPersonBP/Blueprints/ThirdPersonCharacter.ThirdPersonCharacter_C|GetCurrentBoxCarrying _asthird_person_character)
        (:Is%20Valid
          (Variables|Default|SetBox%20on%20platform (Variables|/Game/ThirdPersonBP/Blueprints/ThirdPersonCharacter.ThirdPersonCharacter_C|GetCurrentBoxCarrying _asthird_person_character))
          (Variables|/Game/ThirdPersonBP/Blueprints/ThirdPersonCharacter.ThirdPersonCharacter_C|SetCurrentBoxCarrying _asthird_person_character 0)
          (Transformation|DetachFromActor (Variables|Default|GetBox%20on%20platform) "KeepRelative" "KeepRelative" "KeepRelative")
          (Transformation|SetActorLocation (Variables|Default|GetBox%20on%20platform) (Transformation|GetActorLocation) false false)
          (Development|PrintString "Box plased on platform"))
        (:Is%20Not%20Valid
          (Development|PrintString "No box in character"))))
    (:CastFailed
      (Development|PrintString "Overlap was not character"))))

(fn ConstructionScript)